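; Chat player controller that spawns networking helper actors and lists chat messages in the chat widget.
; BeginPlay spawns a BP_Client on every instance, then on authority only spawns a Server actor and caches the chat widget from BP_ChattingHUD.
; ListMessage creates a WBP_List entry prefixed with the display name of the controller's owner and appends it to the chat widget's scroll box.
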(event `self.ReceiveBeginPlay`
  (bind _returnvalue (`|SpawnActorFromClass` "/Game/Blueprint/BP_Client.BP_Client_C" (`KismetMathLibrary.MakeTransform` (0.0 0.0 0.0)) "Undefined" "OverrideRootScale" null null))
  (set `self.ClientRef` _returnvalue)
  (`/Engine/EditorBlueprintResources/ActorMacros.Switch Has Authority`
    (:`Authority`
      (bind _returnvalue_2 (`|SpawnActorFromClass` "/Script/SocketChatting.Server" (`KismetMathLibrary.MakeTransform` (0.0 0.0 0.0)) "Undefined" "OverrideRootScale" null null))
      (set `self.ServerRef` _returnvalue_2)
      (bind _asbp_chatting_hud (cast `/Game/Blueprint/BP_ChattingHUD` (`self.GetHUD`)))
      (set `self.WBP Chat Ref` (`/Game/Blueprint/BP_ChattingHUD.WBP_ChatRef` _asbp_chatting_hud)))))

(event `/Game/Blueprint/BP_ChatInterface.ListMessage`
  (params (message :type String))
  (bind _returnvalue (`|CreateWidget` "/Game/Widget/WBP_List.WBP_List_C"))
  (set `TextBlock.Text` (`KismetTextLibrary.Conv_StringToText` (`KismetStringLibrary.Concat_StrStr` (`KismetSystemLibrary.GetDisplayName` (`self.GetOwner`)) ": " message)) (`/Game/Widget/WBP_List.Text` _returnvalue))
  (`PanelWidget.AddChild` (`/Game/Widget/WBP_Chat.ScrollBox` (`self.WBP Chat Ref`)) _returnvalue))

(fn `UserConstructionScript`)